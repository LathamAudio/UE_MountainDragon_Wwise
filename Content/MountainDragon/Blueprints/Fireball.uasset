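; Fireball actor for the MountainDragon content that plays a looping or travel sound and explodes when it hits something.
; On BeginPlay it starts its attached audio component and posts the Wwise fireball event on its AkComponent.
; On Hit it spawns an explosion emitter and both explosion sounds at the hit location, stops both attached sources and destroys itself.
; Audio runs through native Unreal and Wwise in parallel.
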(event Collision|EventHit
  (params (MyComp :type Primitive%20Component%20Object%20Reference) (Other :type Actor%20Object%20Reference) (OtherComp :type Primitive%20Component%20Object%20Reference) (bSelfMoved :type Boolean) (HitLocation :type Vector :default "0, 0, 0") (HitNormal :type Vector :default "0, 0, 0") (NormalImpulse :type Vector :default "0, 0, 0") (Hit :type Hit%20Result%20Structure%20%28by%20ref%29))
  (Effects|SpawnEmitteratLocation "/Game/Realistic_Starter_VFX_Pack_Vol2/Particles/Explosion/P_Explosion_Big_B.P_Explosion_Big_B" HitLocation)
  (Audio|PlaySoundatLocation "/Game/MountainDragon/Audio/Metasounds/MSS_MB_Explosion.MSS_MB_Explosion" HitLocation "0, 0, 0" 1.0 1.0 0.0 0 0 0 0)
  (Class|AkGameplayStatics|PostEventatLocation "/Game/WwiseAudio/Events/Play_MB_Explosion.Play_MB_Explosion" HitLocation "0, 0, 0")
  (Audio|Components|Audio|Stop (Variables|Default|GetAttachedAudio))
  (Class|AkGameObject|Stop (Variables|Default|GetAttachedAkComponent))
  (Actor|DestroyActor))

(event Collision|EventActorBeginOverlap
  (params (OtherActor :type Actor%20Object%20Reference)))

(event EventTick
  (params (DeltaSeconds :type Float%20%28single-precision%29)))

(event EventBeginPlay
  (Audio|Components|Audio|Play (Variables|Default|GetAttachedAudio) 0.0)
  (Class|AkGameObject|PostAkEvent (Variables|Default|GetAttachedAkComponent) "/Game/WwiseAudio/Events/Play_MB_Fireball.Play_MB_Fireball"))

(fn ConstructionScript)